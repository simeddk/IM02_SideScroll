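; Boss character that approaches and attacks the player along the Y axis, showing a health HUD once engaged.
; Tick drives a state machine; attacks pick a punch montage, or a flex-then-swipe skill once a one-second timer counter passes a random threshold.
; Externally called events toggle separate punch and skill hitboxes and end attacks.
; Damage updates HUD health via OnRep, flashes a dynamic material red, and triggers death and delayed destruction.
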(event `self.ReceiveBeginPlay`
  ;[1 1 1] 다이나믹 머티리얼 세팅
  (bind _returnvalue (`KismetMaterialLibrary.CreateDynamicMaterialInstance` "/Game/Mixamo/Mutant/Mesh/mutant_M_Inst.mutant_M_Inst"))
  (bind _output_get (set `self.DynamicMaterial` _returnvalue))
  (`PrimitiveComponent.SetMaterial` (`self.Mesh`) 0 _output_get)
  ;[1 1 1] 무기 충돌체 끄기
  (`PrimitiveComponent.SetCollisionEnabled` (`self.PunchCollision`) "NoCollision")
  (`PrimitiveComponent.SetCollisionEnabled` (`self.SkillCollision`) "NoCollision")
  ;[1 1 1] 스킬 타임 증가
  (`KismetSystemLibrary.K2_SetTimerDelegate` (delegate `IncreaseSkillTime`) 1.0 true)
  (set `self.HP` (`self.MaxHP`))
  (`/Game/Game/BP_GameInstance.ShowBossHUD` (`/Game/Game/BP_FunctionLibrary.GetMyGameInstance`) false))

(event `IncreaseSkillTime`
  ;[1 1 1] 스킬 타임 증가
  (`/Engine/EditorBlueprintResources/StandardMacros.IncrementFloat` (`self.SkillTime`)))

(event `self.ReceiveAnyDamage`
  (params (Damage :type "Float (single-precision)") (DamageType :type "DamageType Object Reference") (InstigatedBy :type "Controller Object Reference") (DamageCauser :type "Actor Object Reference"))
  ;[1 1 1] 피격 시
  (`|ExecutionSequence`
    (:`then_0`
      (bind _output_get (set `self.HP` (- (`self.HP`) Damage)))
      (if (<= _output_get 0.0)
        (set `self.StateType` "NewEnumerator3")
        (`self.PlayAnimMontage` "/Game/Mixamo/Mutant/Animations/mutant_dying_Montage.mutant_dying_Montage" 1.0 "Start")
        (`PrimitiveComponent.SetCollisionEnabled` (`self.CapsuleComponent`) "NoCollision")
        (`PrimitiveComponent.SetCollisionEnabled` (`self.PunchCollision`) "NoCollision")
        (`PrimitiveComponent.SetCollisionEnabled` (`self.SkillCollision`) "NoCollision")))
    (:`then_1`
      (`self.HitEffect`))))

(event `HitEffect`
  ;[1 1 1] 피격 시
  (`GameplayStatics.SpawnEmitterAttached` "/Game/InfinityBladeEffects/Effects/FX_Mobile/Fire/combat/P_FireBall_Powerup.P_FireBall_Powerup" (`self.CapsuleComponent`))
  (`GameplayStatics.PlaySoundAtLocation` "/Game/Sounds/Hit.Hit" (`self.K2_GetActorLocation`) (struct) 1.0 1.0 0.0 null null null)
  (`MaterialInstanceDynamic.SetVectorParameterValue` (`self.DynamicMaterial`) "HitColor" (struct :`R` 1.0 :`A` 1.0))
  (`KismetSystemLibrary.Delay` 0.1)
  (`MaterialInstanceDynamic.SetVectorParameterValue` (`self.DynamicMaterial`) "HitColor" (struct :`A` 1.0)))

(event `self.ReceiveTick`
  (params (DeltaSeconds :type "Float (single-precision)"))
  (bind (_returnvalue_x _returnvalue_y) (`KismetMathLibrary.BreakVector` (- (`self.K2_GetActorLocation` (`GameplayStatics.GetPlayerCharacter` 0)) (`self.K2_GetActorLocation`))))
  (bind _returnvalue (`KismetMathLibrary.MakeVector` 0.0 _returnvalue_y))
  ;[1 1 1] 틱 - 상태변경
  (if (not (`self.IsPlayerDead`))
    (set `self.DistanceToPlayer` (`KismetMathLibrary.VSize` _returnvalue))
    (set `self.DirectionToPlayer` (`KismetMathLibrary.Vector_Normal2D` _returnvalue))
    (switch `/Game/Enums/EStateType` (`self.StateType`)
      (:`NewEnumerator0`
        (if (<= (`self.DistanceToPlayer`) 500.0)
          (set `self.StateType` "NewEnumerator1")
          (`/Game/Game/BP_GameInstance.ShowBossHUD` (`/Game/Game/BP_FunctionLibrary.GetMyGameInstance`) true)))
      (:`NewEnumerator1`
        (if (<= (`self.DistanceToPlayer`) (`self.AttackRange`))
          (`self.StartAttack`)
          (else
            (`self.AddMovementInput` (`self.DirectionToPlayer`)))))
      (:`NewEnumerator2`
        (if (`self.bAttacking`)
          _
          (elif (> (`self.DistanceToPlayer`) (`self.AttackRange`))
            (set `self.StateType` "NewEnumerator1"))))
      (:`NewEnumerator3`
        (`KismetSystemLibrary.Delay` 5.0)
        (`/Game/Game/BP_GameInstance.ShowBossHUD` (`/Game/Game/BP_FunctionLibrary.GetMyGameInstance`) false)
        (`self.K2_DestroyActor`)))))

(event `EndAttack`
  ;[1 1 1] 공격 종료 - 멀어지면 쫓아가거나 or 가까우면 재공격
  (if (not (`self.IsPlayerDead`))
    (set `self.bAttacking` false)
    (if (> (`self.DistanceToPlayer`) (`self.AttackRange`))
      (set `self.StateType` "NewEnumerator1")
      (else
        (`self.StartAttack`)))))

(event `self.PunchCollision.OnComponentBeginOverlap`
  (params (OverlappedComponent :type "PrimitiveComponent Object Reference") (OtherActor :type "Actor Object Reference") (OtherComp :type "PrimitiveComponent Object Reference") (OtherBodyIndex :type Integer) (bFromSweep :type Boolean) (SweepResult :type "HitResult Structure (by ref)"))
  ;[1 1 1] 무기에 충돌된 액터에게 대미지 주기
  (if (`/Game/Game/BP_FunctionLibrary.Is Body Tag Valid` OtherComp)
    (if (!= OtherActor self)
      (bind _asbp_player (cast `/Game/Player/BP_Player` OtherActor))
      (`GameplayStatics.ApplyDamage` _asbp_player (`self.Atk`) null self))))

(event `self.SkillCollision.OnComponentBeginOverlap`
  (params (OverlappedComponent :type "PrimitiveComponent Object Reference") (OtherActor :type "Actor Object Reference") (OtherComp :type "PrimitiveComponent Object Reference") (OtherBodyIndex :type Integer) (bFromSweep :type Boolean) (SweepResult :type "HitResult Structure (by ref)"))
  ;[1 1 1] 무기에 충돌된 액터에게 대미지 주기
  (if (`/Game/Game/BP_FunctionLibrary.Is Body Tag Valid` OtherComp)
    (if (!= OtherActor self)
      (bind _asbp_player (cast `/Game/Player/BP_Player` OtherActor))
      (`GameplayStatics.ApplyDamage` _asbp_player (`self.SkillAtk`) null self))))

(event `OnPunchCollision`
  ;[1 1 1] 펀치 충돌체 켜고/끄기
  (`PrimitiveComponent.SetCollisionEnabled` (`self.PunchCollision`) "QueryAndPhysics"))

(event `OnSkillCollision`
  ;[1 1 1] 스킬 충돌체 켜고/끄기
  (`PrimitiveComponent.SetCollisionEnabled` (`self.SkillCollision`) "QueryAndPhysics"))

(event `OffPunchCollision`
  ;[1 1 1] 펀치 충돌체 켜고/끄기
  (`PrimitiveComponent.SetCollisionEnabled` (`self.PunchCollision`) "NoCollision"))

(event `OffSkillCollision`
  ;[1 1 1] 스킬 충돌체 켜고/끄기
  (`PrimitiveComponent.SetCollisionEnabled` (`self.SkillCollision`) "NoCollision"))

(event `StartAttack`
  ;[1 1 1] 공격 분기 - 펀치냐 스킬이냐
  (if (`|EnumInequality` (`self.StateType`) "NewEnumerator3")
    (`self.K2_SetActorRotation` (`KismetMathLibrary.Conv_VectorToRotator` (`self.DirectionToPlayer`)))
    (set `self.bAttacking` true)
    (if (>= (`self.SkillTime`) (`KismetMathLibrary.RandomFloatInRange` 3.0 6.0))
      (set `self.StateType` "NewEnumerator4")
      (`self.PlayAnimMontage` "/Game/Mixamo/Mutant/Animations/mutant_flexing_muscles_Montage.mutant_flexing_muscles_Montage" 3.0 "Start")
      (`KismetSystemLibrary.Delay` 0.5)
      (if (> (`self.HP`) 0.0)
        (`self.PlayAnimMontage` "/Game/Mixamo/Mutant/Animations/mutant_swiping_Montage.mutant_swiping_Montage" 2.0 "None")
        (set `self.SkillTime` 0.0))
      (else
        (set `self.StateType` "NewEnumerator2")
        (`self.PlayAnimMontage` "/Game/Mixamo/Mutant/Animations/Right_Hook_Montage.Right_Hook_Montage")))))

(fn `IsPlayerDead`
  (returns (bDead :type Boolean))
  (bind _asbp_player (cast `/Game/Player/BP_Player` (`GameplayStatics.GetPlayerCharacter` 0)))
  (return (`/Game/Player/BP_Player.bDead` _asbp_player)))

(fn `OnRep_HP`
  (`/Game/UI/WB_PlayHUD.UpdateBossHealth` (`/Game/Game/BP_GameInstance.PlayHUDWidget` (`/Game/Game/BP_FunctionLibrary.GetMyGameInstance`)) (`self.HP`) (`self.MaxHP`)))

(fn `UserConstructionScript`)