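; BP_Potion is a health potion actor that can restore a player's HP.
; On BeginPlay, the RoundTrip timeline lerps its location between the spawn point and a point slightly along its up vector.
; IncreaseHP adds Amount to the given player's HP, clamped between zero and MaxHP, but nothing in this file calls it.
; A disconnected branch that sets the timeline's play rate never runs.
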(event `self.ReceiveBeginPlay`
  (bind _output_get (set `self.Start` (`self.K2_GetActorLocation`)))
  (set `self.End` (+ _output_get (* (`self.GetActorUpVector`) 30)))
  (bind (_direction _alpha) (`Timeline|RoundTrip`)
    (:`Update`
      (`self.K2_SetActorLocation` (`KismetMathLibrary.VLerp` (`self.Start`) (`self.End`) _alpha)))))

(fn `IncreaseHP`
  (params (Player :type "/Game/Player/BP_Player Object Reference"))
  (set `/Game/Player/BP_Player.HP` (`KismetMathLibrary.FClamp` (+ (`/Game/Player/BP_Player.HP` Player) (`self.Amount`)) 0.0 (`/Game/Player/BP_Player.MaxHP` (`local.Player`))) (`local.Player`)))

(fn `UserConstructionScript`)