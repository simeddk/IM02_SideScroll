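; Cinematic trigger that plays the Master_Sequence level sequence once, when BP_Player first overlaps it.
; On overlap it reveals the player and boss cinematic actors (hidden since BeginPlay), disables player input and starts the sequence.
; It then scans all actors, hiding and stopping tick on every Character and BP_EnemyHP.
; The sequence's OnFinished event destroys the cinematic actors, re-enables input and restores visibility and tick.
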(event `self.ReceiveBeginPlay`
  (`self.SetActorHiddenInGame` (`self.CinematicCharacter_Player`) true)
  (`self.SetActorHiddenInGame` (`self.CinematicCharacter_Boss`) true))

(event `self.ReceiveActorBeginOverlap`
  (params (OtherActor :type "Actor Object Reference"))
  (cast `/Game/Player/BP_Player` OtherActor)
  (`/Engine/EditorBlueprintResources/StandardMacros.DoOnce` false
    (:`Completed`
      (`self.SetActorHiddenInGame` (`self.CinematicCharacter_Player`) false)
      (`self.SetActorHiddenInGame` (`self.CinematicCharacter_Boss`) false)
      (`self.DisableInput` (`GameplayStatics.GetPlayerCharacter` 0) (`GameplayStatics.GetPlayerController` 0))
      (bind (_outactor _returnvalue) (`LevelSequencePlayer.CreateLevelSequencePlayer` "/Game/Cinematices/Master_Sequence.Master_Sequence"))
      (add `MovieSceneSequencePlayer.OnFinished` _returnvalue (delegate `OnFinished`))
      (`MovieSceneSequencePlayer.Play` _returnvalue)
      (bind _outactors (`GameplayStatics.GetAllActorsOfClass` "/Script/Engine.Actor"))
      (for _array_element _outactors
        (bind _returnvalue_2 (`GameplayStatics.GetObjectClass` _array_element))
        (if (or (`KismetMathLibrary.ClassIsChildOf` _returnvalue_2 "/Script/Engine.Character") (`KismetMathLibrary.ClassIsChildOf` _returnvalue_2 "/Game/Enemy/BP_EnemyHP.BP_EnemyHP_C"))
          (`self.SetActorHiddenInGame` _array_element true)
          (`self.SetActorTickEnabled` _array_element false))))))

(event `OnFinished`
  (`self.K2_DestroyActor` (`self.CinematicCharacter_Player`))
  (`self.K2_DestroyActor` (`self.CinematicCharacter_Boss`))
  (`self.EnableInput` (`GameplayStatics.GetPlayerCharacter` 0) (`GameplayStatics.GetPlayerController` 0))
  (bind _outactors (`GameplayStatics.GetAllActorsOfClass` "/Script/Engine.Actor"))
  (for _array_element _outactors
    (bind _returnvalue (`GameplayStatics.GetObjectClass` _array_element))
    (if (or (`KismetMathLibrary.ClassIsChildOf` _returnvalue "/Script/Engine.Character") (`KismetMathLibrary.ClassIsChildOf` _returnvalue "/Game/Enemy/BP_EnemyHP.BP_EnemyHP_C"))
      (`self.SetActorHiddenInGame` _array_element false)
      (`self.SetActorTickEnabled` _array_element true))))

(fn `UserConstructionScript`)